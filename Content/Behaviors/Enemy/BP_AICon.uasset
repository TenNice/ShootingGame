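; AI controller for enemies that runs BT_Enemy on possess and selects targets through AI perception.
; A sensed Player-tagged actor takes priority, setting the pawn's Target once per sighting and updating the blackboard's HasLineOfSight and EnemyActor.
; Other updates start a one-second lost-player timer while the player counts as seen.
; Once DoNotSeePlayer is set, they set Target and engage only BP_PlaneBox actors with Check2 false.
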(event OnTargetPerceptionUpdated(AIPerception)
  (params (Actor :type Actor%20Object%20Reference) (Stimulus :type AI%20Stimulus%20Structure))
  (bind _blackboard (Variables|Default|GetBlackboard))
  (bind _blackboard_2 (Variables|Default|GetBlackboard))
  (bind _blackboard_3 (Variables|Default|GetBlackboard))
  (bind _blackboard_4 (Variables|Default|GetBlackboard))
  (if (and (Actor|ActorHasTag Actor "Player") (.bSuccessfullySensed (Utilities|Struct|BreakAIStimulus Stimulus)))
    (Utilities|FlowControl|Sequence
      (:then_0
        (Utilities|FlowControl|DoOnce false
          (:Completed
            (Variables|Default|SetDoNotSeePlayer false)
            ;[1 1 1] 인지한 타겟이 무엇인지 BP_Enemy에 넘겨주는 부분
            (bind _output_get (Variables|/Game/Blueprints/Characters/BP_Enemy.BP_Enemy_C|SetTarget (.AsBP%20Enemy (Utilities|Casting|CastToBP_Enemy (Pawn|GetControlledPawn))) Actor))
            (Development|PrintString (Utilities|GetDisplayName _output_get)))))
      (:then_1
        (Utilities|Time|ClearandInvalidateTimerbyHandle (Variables|Default|GetTimerHandle))
        (AI|Components|Blackboard|SetValueasBool _blackboard_3 (Variables|Default|GetHasLineOfSight) true)
        (AI|Components|Blackboard|SetValueasObject _blackboard_3 (Variables|Default|GetEnemyActor) Actor)))
    (elif (Variables|Default|GetDoNotSeePlayer)
      ;[1 1 1] 인지한 타겟이 무엇인지 BP_Enemy에 넘겨주는 부분
      (bind _output_get_2 (Variables|/Game/Blueprints/Characters/BP_Enemy.BP_Enemy_C|SetTarget (.AsBP%20Enemy (Utilities|Casting|CastToBP_Enemy (Pawn|GetControlledPawn))) Actor))
      (Development|PrintString (Utilities|GetDisplayName _output_get_2))
      (bind _asbp_plane_box (Utilities|Casting|CastToBP_PlaneBox Actor)
        (:then
          ;[1 1 1] 블럭 색 확인
          (if (Variables|/Game/Blueprints/BP_PlaneBox.BP_PlaneBox_C|GetCheck2 _asbp_plane_box)
            (AI|Components|Blackboard|SetValueasBool _blackboard (Variables|Default|GetHasLineOfSight) false)
            (AI|Components|Blackboard|SetValueasObject _blackboard (Variables|Default|GetEnemyActor) 0)
            (else
              (AI|Components|Blackboard|SetValueasBool _blackboard_4 (Variables|Default|GetHasLineOfSight) true)
              (AI|Components|Blackboard|SetValueasObject _blackboard_4 (Variables|Default|GetEnemyActor) Actor))))
        (:CastFailed
          (AI|Components|Blackboard|SetValueasBool _blackboard_2 (Variables|Default|GetHasLineOfSight) false)
          (AI|Components|Blackboard|SetValueasObject _blackboard_2 (Variables|Default|GetEnemyActor) 0)))
      (else
        (bind _returnvalue (Utilities|Time|SetTimerbyEvent (delegate Custom|LostPlayer) 1.0))
        (Variables|Default|SetTimerHandle _returnvalue)))))

(event Custom|LostPlayer
  (Variables|Default|SetDoNotSeePlayer true)
  (Utilities|FlowControl|DoOnce false) ; enters at Reset
)

(event EventBeginPlay)

(event EventTick
  (params (DeltaSeconds :type Float%20%28single-precision%29)))

(event EventPossess
  (params (PossessedPawn :type Pawn%20Object%20Reference))
  (AI|RunBehaviorTree "/Game/Behaviors/Enemy/BT_Enemy.BT_Enemy"))

(fn ConstructionScript)