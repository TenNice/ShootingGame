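; BP_Bullet is a projectile actor that damages BP_Enemy actors it overlaps.
; On BeginPlay it takes its direction from the instigator controller's forward vector and sets a short lifespan.
; Tick moves it along that vector at BulletSpeed by setting its location directly, without sweep.
; Overlapping an enemy applies fixed damage, spawns an explosion emitter and destroys the bullet, while other actors are ignored.
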(event EventBeginPlay
  (Variables|Default|SetBulletVector (Transformation|GetActorForwardVector (Game|GetInstigatorController)))
  (Actor|SetLifeSpan 3.0))

(event EventTick
  (params (DeltaSeconds :type Float%20%28single-precision%29))
  (Transformation|SetActorLocation (+ (Transformation|GetActorLocation) (* (* (Variables|Default|GetBulletVector) (Variables|Default|GetBulletSpeed)) DeltaSeconds)) false false))

(event Collision|EventActorBeginOverlap
  (params (OtherActor :type Actor%20Object%20Reference))
  (bind _asbp_enemy (Utilities|Casting|CastToBP_Enemy OtherActor))
  (Game|Damage|ApplyDamage _asbp_enemy 1e+01 0 0)
  (Effects|SpawnEmitteratLocation "/Game/StarterContent/Particles/P_Explosion.P_Explosion" (Transformation|GetActorLocation))
  (Actor|DestroyActor))

(fn ConstructionScript)