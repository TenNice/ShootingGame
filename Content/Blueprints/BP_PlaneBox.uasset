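; BP_PlaneBox is a box of six plane meshes that bullets claim for one of two sides by recoloring it.
; On overlap, a BP_Bullet turns all faces blue and sets Count to 1, while a BP_Bullet_Enemy turns them red and sets Count to -1.
; The Check1 and Check2 flags track the current color, so repeat hits from the same side do nothing.
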(event EventBeginPlay)

(event Collision|EventActorBeginOverlap
  (params (OtherActor :type Actor%20Object%20Reference))
  (Utilities|Casting|CastToBP_Bullet OtherActor
    (:then
      (if (not (Variables|Default|GetCheck1))
        (Variables|Default|SetCheck1 true)
        (Variables|Default|SetCheck2 false)
        (Variables|Default|SetCount 1)
        (Rendering|Material|SetMaterial (Variables|Default|GetPlaneBottom_StaticMeshComponent0) 0 "/Game/Materials/M_Plane_InstBlue.M_Plane_InstBlue")
        (Rendering|Material|SetMaterial (Variables|Default|GetPlane1_StaticMeshComponent0) 0 "/Game/Materials/M_Plane_InstBlue.M_Plane_InstBlue")
        (Rendering|Material|SetMaterial (Variables|Default|GetPlane2_StaticMeshComponent0) 0 "/Game/Materials/M_Plane_InstBlue.M_Plane_InstBlue")
        (Rendering|Material|SetMaterial (Variables|Default|GetPlane3_StaticMeshComponent0) 0 "/Game/Materials/M_Plane_InstBlue.M_Plane_InstBlue")
        (Rendering|Material|SetMaterial (Variables|Default|GetPlane4_StaticMeshComponent0) 0 "/Game/Materials/M_Plane_InstBlue.M_Plane_InstBlue")
        (Rendering|Material|SetMaterial (Variables|Default|GetPlaneTop_StaticMeshComponent0) 0 "/Game/Materials/M_Plane_InstBlue.M_Plane_InstBlue")))
    (:CastFailed
      (Utilities|Casting|CastToBP_Bullet_Enemy OtherActor)
      (if (not (Variables|Default|GetCheck2))
        (Variables|Default|SetCheck2 true)
        (Variables|Default|SetCheck1 false)
        (Variables|Default|SetCount -1)
        (Rendering|Material|SetMaterial (Variables|Default|GetPlaneBottom_StaticMeshComponent0) 0 "/Game/Materials/M_Plane_InstRed.M_Plane_InstRed")
        (Rendering|Material|SetMaterial (Variables|Default|GetPlane1_StaticMeshComponent0) 0 "/Game/Materials/M_Plane_InstRed.M_Plane_InstRed")
        (Rendering|Material|SetMaterial (Variables|Default|GetPlane2_StaticMeshComponent0) 0 "/Game/Materials/M_Plane_InstRed.M_Plane_InstRed")
        (Rendering|Material|SetMaterial (Variables|Default|GetPlane3_StaticMeshComponent0) 0 "/Game/Materials/M_Plane_InstRed.M_Plane_InstRed")
        (Rendering|Material|SetMaterial (Variables|Default|GetPlane4_StaticMeshComponent0) 0 "/Game/Materials/M_Plane_InstRed.M_Plane_InstRed")
        (Rendering|Material|SetMaterial (Variables|Default|GetPlaneTop_StaticMeshComponent0) 0 "/Game/Materials/M_Plane_InstRed.M_Plane_InstRed")))))

(event EventTick
  (params (DeltaSeconds :type Float%20%28single-precision%29)))

(fn ConstructionScript)