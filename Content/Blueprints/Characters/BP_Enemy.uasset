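; Enemy character Blueprint that shoots at a Target actor and dies when its HP runs out.
; Fire spawns an enemy bullet slightly ahead of the enemy, rotated by look-at toward Target's current location.
; AnyDamage subtracts from HP, while Tick polls it and destroys the actor at zero or below.
; UpdateWalkSpeed sets the movement component's max walk speed; leftover blackboard and forward-firing nodes are disconnected.
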(event Custom|Fire
  (bind _returnvalue (Transformation|GetActorLocation))
  (bind _target (Variables|Default|GetTarget))
  (bind _returnvalue_2 (Transformation|GetActorLocation _target))
  (bind _returnvalue_3 (Math|Rotator|FindLookatRotation _returnvalue _returnvalue_2))
  (Game|SpawnActorfromClass "/Game/Blueprints/BP_Bullet_Enemy.BP_Bullet_Enemy_C" (Math|Transform|MakeTransform (+ _returnvalue (* (Math|Vector|GetForwardVector _returnvalue_3) 1e+02)) _returnvalue_3 "1.000000,1.000000,1.000000") "AlwaysSpawn" 0 0))

(event Game|Damage|EventAnyDamage
  (params (Damage :type Float%20%28single-precision%29) (DamageType :type Damage%20Type%20Object%20Reference) (InstigatedBy :type Controller%20Object%20Reference) (DamageCauser :type Actor%20Object%20Reference))
  (Variables|Default|SetHP (- (Variables|Default|GetHP) Damage)))

(event Collision|EventActorBeginOverlap
  (params (OtherActor :type Actor%20Object%20Reference)))

(event EventTick
  (params (DeltaSeconds :type Float%20%28single-precision%29))
  (if (<= (Variables|Default|GetHP) 0.0)
    (Actor|DestroyActor)))

(fn ConstructionScript)

(fn UpdateWalkSpeed
  (params (최대%20걷기%20속도 :type Float%20%28single-precision%29))
  (Variables|/Script/Engine.CharacterMovementComponent|SetMaxWalkSpeed (Variables|Character|GetCharacterMovement) 최대%20걷기%20속도))