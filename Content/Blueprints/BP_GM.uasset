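; BP_GM ends the match after a fixed 20-second timer and decides whether the player wins or loses.
; Tick accumulates game time, then a DoOnce loops over every BP_PlaneBox, summing Count into Win.
; The loop body also creates a UMG_EndGame widget per box and hits a one-second Delay.
; After the delay it removes the widget and calls EndGameWin on BP_PC if Win is positive, otherwise EndGameLose.
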(event EventBeginPlay)

(event EventTick
  (params (DeltaSeconds :type Float%20%28single-precision%29))
  (bind _output_get (Variables|Default|SetGameTime (+ DeltaSeconds (Variables|Default|GetGameTime))))
  (if (> _output_get 2e+01)
    (Utilities|FlowControl|DoOnce false
      (:Completed
        ;[1 1 1] 어느 팀이 이겼는지 계산
        (bind _outactors (Actor|GetAllActorsOfClass "/Game/Blueprints/BP_PlaneBox.BP_PlaneBox_C"))
        (for _array_element _outactors
          (bind _output_get_2 (Variables|Default|SetWin (+ (Variables|/Game/Blueprints/BP_PlaneBox.BP_PlaneBox_C|GetCount _array_element) (Variables|Default|GetWin))))
          (bind _asbp_pc (Utilities|Casting|CastToBP_PC (Game|GetPlayerController 0)))
          (bind _returnvalue (UserInterface|CreateWidget "/Game/UMGs/UMG_EndGame.UMG_EndGame_C" _asbp_pc))
          (UserInterface|Viewport|AddtoViewport _returnvalue 0)
          (Utilities|FlowControl|Delay 1.0)
          (Widget|RemovefromParent _returnvalue)
          (if (> _output_get_2 0)
            (bind _asbp_pc_2 (Utilities|Casting|CastToBP_PC (Game|GetPlayerController 0)))
            (Default|EndGameWin _asbp_pc_2)
            (else
              (bind _asbp_pc_3 (Utilities|Casting|CastToBP_PC (Game|GetPlayerController 0)))
              (Default|EndGameLose _asbp_pc_3))))))))

(fn ConstructionScript)