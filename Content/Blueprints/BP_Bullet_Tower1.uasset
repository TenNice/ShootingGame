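; BP_Bullet_Tower1 is a projectile actor, named as the bullet for Tower 1.
; On BeginPlay it caches its forward vector and sets a short lifespan, then moves along that vector each Tick at BulletSpeed without sweeping.
; Any actor overlap spawns an explosion particle effect at its location and destroys the bullet, with no damage applied in this Blueprint.
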(event EventBeginPlay
  (Variables|Default|SetBulletVector (Math|Vector|GetForwardVector (Transformation|GetActorRotation)))
  (Actor|SetLifeSpan 3.0))

(event EventTick
  (params (DeltaSeconds :type Float%20%28single-precision%29))
  (Transformation|SetActorLocation (+ (Transformation|GetActorLocation) (* (* (Variables|Default|GetBulletVector) (Variables|Default|GetBulletSpeed)) DeltaSeconds)) false false))

(event Collision|EventActorBeginOverlap
  (params (OtherActor :type Actor%20Object%20Reference))
  (Effects|SpawnEmitteratLocation "/Game/StarterContent/Particles/P_Explosion.P_Explosion" (Transformation|GetActorLocation))
  (Actor|DestroyActor))

(fn ConstructionScript)